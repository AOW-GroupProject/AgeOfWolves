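; Gameplay ability for the AkaOni player that handles unequipping the weapon by signalling a combat state change.
; On activation it commits the ability cost and, on success, sends the OnChangeCombatState gameplay event, with debug prints along the way.
; It ends immediately whether or not the commit succeeds.
; A disconnected, unfinished branch that reads CurrentCombatState from BaseAttributeSet never runs.
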(event Ability|EventActivateAbility
  (bind _returnvalue (Ability|CommitAbilityCost false))
  (Development|PrintString (Utilities|String|ToString(Boolean) _returnvalue))
  (if _returnvalue
    (Ability|SendGameplayEvent "(TagName=\"EventTag.OnChangeCombatState\")")
    (Development|PrintString "Unequip")
    (Ability|EndAbility)
    (else
      (Ability|EndAbility))))