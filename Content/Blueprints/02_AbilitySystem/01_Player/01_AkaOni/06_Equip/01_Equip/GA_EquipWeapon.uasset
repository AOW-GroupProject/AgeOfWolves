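; GA_EquipWeapon is a gameplay ability that plays the Aka Oni player's weapon equip montage.
; On activation it proceeds only if the owner's BaseAttributeSet reports a combat state of zero and the ability cost commits, otherwise it ends.
; When the montage completes it sends the OnChangeCombatState gameplay event and ends; a cancelled montage ends it without the event.
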(event Ability|EventActivateAbility
  (bind _returnvalue (Ability|GetAbilitySystemComponentfromActorInfo))
  (Utilities|IsValid _returnvalue
    (:Is%20Valid
      (bind _returnvalue_2 (GameplayAttributes|GetAttributeSet _returnvalue "/Script/AgeOfWolves.BaseAttributeSet"))
      (bind _asbase_attribute_set (Utilities|Casting|CastToBaseAttributeSet _returnvalue_2)
        (:then
          (Utilities|IsValid _asbase_attribute_set
            (:Is%20Valid
              (if (== 0.0 (Class|BaseAttributeSet|GetCurrentCombatState _asbase_attribute_set))
                (bind _returnvalue_3 (Ability|CommitAbilityCost false))
                (Development|PrintString (Utilities|String|ToString(Boolean) _returnvalue_3))
                (if _returnvalue_3
                  (|PlayMontageandWaitProxy "None" (Variables|Default|GetEquipMontage) 1.0 "None" true 1.0 0.0
                    (:OnCompleted
                      (Ability|SendGameplayEvent "(TagName=\"EventTag.OnChangeCombatState\")")
                      (Development|PrintString "Equip")
                      (Ability|EndAbility))
                    (:OnCancelled
                      (Ability|EndAbility)))
                  (else
                    (Ability|EndAbility)))
                (else
                  (Ability|EndAbility))))
            (:Is%20Not%20Valid
              (Ability|EndAbility))))
        (:CastFailed
          (Ability|EndAbility))))
    (:Is%20Not%20Valid
      (Ability|EndAbility))))