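; Base gameplay ability for the player's katana combo attack: it turns the player toward a target and plays the first attack montage.
; Montage start and end gameplay events toggle a looping timer that sphere-traces between the blade sockets.
; Each newly hit actor joins an ignore list and receives one damage event; ending the ability clears the list and timer.
; A helper maps combo index to section name, though this graph never calls it.
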(event Custom|Attack%20Trace%20Loop
  ;[1 1 1] 공격 중에 실행되는 Sphere Trace Loop
  (bind (_outhit _returnvalue) (Collision|SphereTraceByChannel (Transformation|GetSocketLocation (Variables|/Script/Engine.Character|GetMesh (Class|AttackGameplayAbility|GetPlayerCharacterfromActorInfo)) "BladeEnd") (Transformation|GetSocketLocation (Variables|/Script/Engine.Character|GetMesh (Class|AttackGameplayAbility|GetPlayerCharacterfromActorInfo)) "BladeStart") (Variables|Default|GetKatanaRadius) "TraceTypeQuery1" false (Variables|Default|GetActorsToIgnore) "None" true "(R=1.000000,G=0.000000,B=0.000000,A=1.000000)" "(R=0.000000,G=1.000000,B=0.000000,A=1.000000)" 2.5))
  (if _returnvalue
    (bind _returnvalue_2 (Utilities|Array|AddUnique (Variables|Default|GetActorsToIgnore) (.HitActor (Collision|BreakHitResult _outhit))))
    (if (>= _returnvalue_2 0)
      (Class|AttackGameplayAbility|SendDamageEvent _outhit))))

(event Custom|Stop%20Attack%20Trace
  ;[1 1 1] 공격 중에 실행되는 Sphere Trace Loop
  (Utilities|Time|ClearandInvalidateTimerbyHandle (Variables|Default|GetKatanaTraceLoop)))

(event Custom|Start%20Attack%20Trace
  ;[1 1 1] 공격 중에 실행되는 Sphere Trace Loop
  (bind _returnvalue (Utilities|Time|SetTimerbyEvent (delegate Custom|Attack%20Trace%20Loop) 0.025 true))
  (Variables|Default|SetKatanaTraceLoop _returnvalue))

(event Ability|EventActivateAbility
  (bind _returnvalue (Class|AttackGameplayAbility|GetPlayerCharacterfromActorInfo))
  ;[1 1 1] 어빌리티 작동
  (bind _returnvalue_2 (Ability|CommitAbility))
  (if _returnvalue_2
    (Utilities|Array|AddUnique (Variables|Default|GetActorsToIgnore) _returnvalue)
    (Utilities|FlowControl|Sequence
      (:then_0
        (Ability|Tasks|WaitGameplayEvent "(TagName=\"EventTag.Montage.Start\")" 0 true
          (:EventReceived
            (CallFunction|StartAttackTrace))))
      (:then_1
        (Ability|Tasks|WaitGameplayEvent "(TagName=\"EventTag.Montage.End\")" 0 true
          (:EventReceived
            (CallFunction|StopAttackTrace))))
      (:then_2
        (Class|PlayerCharacter|UpdateFacingTarget _returnvalue))
      (:then_3
        (|PlayMontageandWaitProxy "" (Utilities|Array|Get(acopy) (Variables|Default|GetAttackMontages)) 1.0 "Default" false 1.0 0.0
          (:OnCompleted
            _)
          (:OnInterrupted
            _)
          (:OnCancelled
            _))
        (Ability|EndAbility)))))

(event Ability|EventOnEndAbility
  (params (bWasCancelled :type Boolean))
  ;[1 1 1] Ability 종료시 필요한 작업을 한다.
  (Utilities|Array|Clear (Variables|Default|GetActorsToIgnore))
  (CallFunction|StopAttackTrace))

(fn GetStartSectionName
  (params (ComboIndex :type Integer))
  (switch int ComboIndex
    (:Default
      _)
    (:0
      _)
    (:1
      _)
    (:2
      (return "2"))
    (:3
      (return "3"))
    (:4
      (return "4")))
  (return "1"))