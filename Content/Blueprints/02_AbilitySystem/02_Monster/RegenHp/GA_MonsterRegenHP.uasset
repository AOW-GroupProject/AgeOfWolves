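; Gameplay ability that, by its name, regenerates monster HP over time.
; After an initial delay, it loops on a WaitDelay task, comparing two float attributes from the owner's BaseAbilitySystemComponent on each pass.
; While the first exceeds the second, it commits the ability cost, apparently using the cost effect as the regen tick, then waits again.
; Otherwise, or if the component is invalid, it ends the ability.
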(event Ability|EventActivateAbility
  (bind _asbase_ability_system_component (Utilities|Casting|CastToBaseAbilitySystemComponent (.AbilitySystemComponent (Utilities|Struct|BreakGameplayAbilityActorInfo (Ability|GetActorInfo)))))
  (Utilities|IsValid _asbase_ability_system_component
    (:Is%20Valid
      (Utilities|FlowControl|Delay 3.0)
      (Ability|Tasks|WaitDelay 5.0 :!label _label
        (:OnFinish
          (if (> (.ReturnValue (Ability|Attribute|GetFloatAttributefromAbilitySystemComponent _asbase_ability_system_component "(AttributeName=\"MaxHealth\",Attribute=/Script/AgeOfWolves.BaseAttributeSet:MaxHealth,AttributeOwner=/Script/CoreUObject.Class'\"/Script/AgeOfWolves.BaseAttributeSet\"')")) (.ReturnValue (Ability|Attribute|GetFloatAttributefromAbilitySystemComponent _asbase_ability_system_component "(AttributeName=\"Health\",Attribute=/Script/AgeOfWolves.BaseAttributeSet:Health,AttributeOwner=/Script/CoreUObject.Class'\"/Script/AgeOfWolves.BaseAttributeSet\"')")))
            (Ability|CommitAbilityCost false)
            (goto _label)
            (else
              (Ability|EndAbility))))))
    (:Is%20Not%20Valid
      (Ability|EndAbility))))