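; Monster gameplay ability for the third basic attack, currently tied to BP_Wolf by a cast on the owner.
; It plays the Wolf_BasicAttack_3 montage and waits once for the Ability.Monster.AttackHit gameplay event.
; On that event it damages the blackboard's Player actor with a calculated hit-direction tag and prints the tag.
; EndAbility runs only when the montage is interrupted or cancelled.
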(event Ability|EventActivateAbility
  (bind _asbp_wolf (Utilities|Casting|CastToBP_Wolf (.owneractor (Ability|GetActorInfo)))) ; 나중에 BaseMonster로 Casting해서 BasicAttack 오버라이드 하도록
  (|PlayMontageandWaitProxy "None" "/Game/TempAsset/Enemy_Bear/Enemy_Bear_Animations/Wolf_BasicAttack_3.Wolf_BasicAttack_3" 1.0 "None" true 1.0 0.0
    (:then
      (Ability|Tasks|WaitGameplayEvent "(TagName=\"Ability.Monster.AttackHit\")" 0 true
        (:EventReceived
          (bind _as액터 (Utilities|Casting|CastToActor (AI|Components|Blackboard|GetValueasObject (AI|GetBlackboard (AI|GetAIController _asbp_wolf)) (Utilities|Name|MakeLiteralName "Player"))))
          (bind _returnvalue (Class|AttackGameplayAbility|CalculateHitDirection (Transformation|GetActorLocation (Ability|GetAvatarActorfromActorInfo))))
          (Class|AttackGameplayAbility|CauseDamagetoTarget _as액터 _returnvalue)
          (Development|PrintString (Utilities|String|ToString(Name) (GameplayTags|GetTagName _returnvalue))) ; 플레이어에게 데미지
        )))
    (:OnInterrupted
      (Ability|EndAbility :!label _label))
    (:OnCancelled
      (goto _label))))

(event Ability|EventOnEndAbility
  (params (bWasCancelled :type Boolean)))