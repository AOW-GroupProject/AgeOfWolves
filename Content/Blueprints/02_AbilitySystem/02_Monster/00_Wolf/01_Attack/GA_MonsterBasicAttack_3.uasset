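; Gameplay ability for the Wolf monster's third basic attack, unfinished: no damage is applied.
; On activation it casts the owner to BP_Wolf, runs a montage task and waits once for the Ability.Monster.AttackHit event.
; On that event it only fetches the Player actor from the AI controller's blackboard.
; The ability ends only when the montage is interrupted or cancelled, with no handling for normal completion.
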(event Ability|EventActivateAbility
  (bind _asbp_wolf (Utilities|Casting|CastToBP_Wolf (.owneractor (Ability|GetActorInfo)))) ; 나중에 BaseMonster로 Casting해서 BasicAttack 오버라이드 하도록
  (|PlayMontageandWaitProxy "None" 0 1.0 "None" true 1.0 0.0
    (:then
      (Ability|Tasks|WaitGameplayEvent "(TagName=\"Ability.Monster.AttackHit\")" 0 true
        (:EventReceived
          (Utilities|Casting|CastToActor (AI|Components|Blackboard|GetValueasObject (AI|GetBlackboard (AI|GetAIController _asbp_wolf)) (Utilities|Name|MakeLiteralName "Player"))))))
    (:OnInterrupted
      (Ability|EndAbility :!label _label))
    (:OnCancelled
      (goto _label))))

(event Ability|EventOnEndAbility
  (params (bWasCancelled :type Boolean)))