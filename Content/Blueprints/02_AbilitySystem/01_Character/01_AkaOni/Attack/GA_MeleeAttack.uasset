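; Gameplay ability for AkaOni's katana melee attack that plays a montage and damages what the blade hits.
; A looping timer sphere-traces between blade sockets, adding hit actors to an ignore list to avoid repeat hits.
; Gameplay events stop the trace, stop the montage when the combat component allows a combo, or reset the combo.
; Ending clears the ignore list because the ability is instanced per actor.
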(event Custom|Attack%20Trace%20Loop
  ;[1 1 1] 공격 중에 실행되는 Sphere Trace Loop
  (bind _outhit (Collision|SphereTraceByChannel (Transformation|GetSocketLocation (Variables|/Script/Engine.Character|GetMesh (Class|AttackGameplayAbility|GetPlayerCharacterfromActorInfo)) "BladeStart") (Transformation|GetSocketLocation (Variables|/Script/Engine.Character|GetMesh (Class|AttackGameplayAbility|GetPlayerCharacterfromActorInfo)) "BladeEnd") (Variables|Default|GetKatanaRadius) "TraceTypeQuery1" false (Variables|Default|GetActorsToIgnore) "None"))
  (if (.bBlockingHit (Collision|BreakHitResult _outhit))
    (Utilities|Array|AddUnique (Variables|Default|GetActorsToIgnore) (.HitActor (Collision|BreakHitResult _outhit)))
    (Class|AttackGameplayAbility|CauseDamage (.HitActor (Collision|BreakHitResult _outhit)))))

(event Custom|Stop%20Trace
  ;[1 1 1] 공격 중에 실행되는 Sphere Trace Loop
  (Utilities|Time|ClearandInvalidateTimerbyHandle (Variables|Default|GetKatanaTraceLoop)))

(event Custom|Start%20Attack%20Trace
  ;[1 1 1] 공격 중에 실행되는 Sphere Trace Loop
  (bind _returnvalue (Utilities|Time|SetTimerbyEvent (delegate Custom|Attack%20Trace%20Loop) 0.05 true))
  (Variables|Default|SetKatanaTraceLoop _returnvalue))

(event Ability|EventActivateAbility
  (bind _returnvalue (Class|AttackGameplayAbility|GetCombatComponentfromPlayerCharacter))
  ;[1 1 1] 코멘트
  (bind _returnvalue_2 (Ability|CommitAbility))
  (if _returnvalue_2
    (Utilities|Array|AddUnique (Variables|Default|GetActorsToIgnore) (Class|AttackGameplayAbility|GetPlayerCharacterfromActorInfo))
    (CallFunction|StartAttackTrace)
    (Utilities|FlowControl|Sequence
      (:then_0
        (Ability|Tasks|WaitGameplayEvent :OptionalExternalTarget 0
          (:EventReceived
            (CallFunction|StopTrace))))
      (:then_1
        (Ability|Tasks|WaitGameplayEvent "(TagName=\"Event.AnimNotify.TriggerCombo\")" 0
          (:EventReceived
            (bind _returnvalue_3 (Class|CombatComponent|CanComboAttack _returnvalue))
            (if _returnvalue_3
              (Animation|Montage|MontageStop -1.0)))))
      (:then_2
        (Ability|Tasks|WaitGameplayEvent "(TagName=\"Event.AnimNotify.ResetCombo\")" 0
          (:EventReceived
            (Class|CombatComponent|ResetCombo _returnvalue)
            (Ability|EndAbility :!label _label))))
      (:then_3
        (|PlayMontageandWaitProxy "" (Utilities|Array|Get(acopy) (Variables|Default|GetMeleeAttackMontages)) 1.0 "" false 1.0 0.0
          (:OnCompleted
            (goto _label))
          (:OnInterrupted
            (goto _label))
          (:OnCancelled
            (goto _label)))))))

(event Ability|EventOnEndAbility
  (params (bWasCancelled :type Boolean))
  ;[1 1 1] Ability의 Instancing Policy가 Instanced Per Actor이기 때문에 이벤트가 종료될 때 초기화 작업을 한다.
  (Utilities|Array|Clear (Variables|Default|GetActorsToIgnore)))