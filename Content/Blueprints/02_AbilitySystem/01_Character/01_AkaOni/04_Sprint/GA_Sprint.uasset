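; GA_Sprint is a Gameplay Ability that lets its owning character sprint at the cost of stamina.
; On activation it applies the move-speed effect GE_Sprint_ChangeMoveSpeed, then briefly waits to confirm horizontal movement.
; A recurring WaitDelay loop commits the ability cost while the owner is accelerating and not falling.
; Input release, stopping, falling or a failed cost sets EndSprint, calls effect removal and ends the ability.
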(event Ability|EventActivateAbility
  (bind _returnvalue (Ability|GetActorInfo))
  (bind (_owneractor _avataractor _playercontroller _abilitysystemcomponent _skeletalmeshcomponent _animinstance _movementcomponent) (Utilities|Struct|BreakGameplayAbilityActorInfo _returnvalue))
  ;[1 1 1] #1. Gameplay Ability의 Owner가 현재 어느 방향으로든 이동 중인지 확인합니다.
  (bind _asbase_character_movement_component (Utilities|Casting|CastToBaseCharacterMovementComponent _movementcomponent))
  (Utilities|IsValid _asbase_character_movement_component
    (:Is%20Valid
      ;[1 1 1] #2. GE_Sprint_ChangeMoveSpeed를 Owner에게 적용하고, 그 반환 값을 통해 Active Gameplay Effect Handle을 설정합니다.
      (bind _returnvalue_2 (Ability|ApplyGameplayEffectToOwner "/Game/Blueprints/02_AbilitySystem/01_Character/01_AkaOni/04_Sprint/GE_Sprint_ChangeMoveSpeed.GE_Sprint_ChangeMoveSpeed_C" (Ability|GetAbilityLevel)))
      (Variables|Default|SetActiveApplyGameplayEffectHandle _returnvalue_2)
      (Utilities|FlowControl|Delay 0.05)
      (if (> (Math|Vector|VectorLengthXY (Transformation|GetVelocity _owneractor)) 0.5)
        ;[1 1 1] #4. Ability Task(Gameplay Ability의 비동기 작업을 수행하는 객체) 중 Wait Delay(Delay 노드랑 같음) 0.05초 주기로 사용자 Key Input 입력이 해제되지 않았다면,
        ; 해당Gameplay Ability의 Owner의 '이동 중' 여부를 체크하고, 이에 대한 GE_Cost_Sprint_DrainStamina(해당 Gameplay Ability 활성화를 위해 필요한 비용)를 Owner에게 부과해줍니다.
        (Ability|Tasks|WaitDelay 0.05 :!label _label
          (:OnFinish
            (bind _asbase_character_movement_component_2 (Utilities|Casting|CastToBaseCharacterMovementComponent (.movementcomponent (Ability|GetActorInfo))))
            (if (and (> (Math|Vector|VectorLength (Pawn|Components|CharacterMovement|GetCurrentAcceleration _asbase_character_movement_component_2)) 0.0) (not (AI|Components|NavMovement|IsFalling _asbase_character_movement_component_2)))
              (bind _returnvalue_3 (Ability|CommitAbilityCost false))
              (if _returnvalue_3
                (if (Variables|Default|GetbEndSprint)
                  _
                  (else
                    (goto _label)))))
            (Variables|Default|SetbEndSprint true)
            (Ability|RemoveGameplayEffectFromOwnerWithHandle (Variables|Default|GetActiveApplyGameplayEffectHandle))
            (Ability|EndAbility)))
        (else
          (Variables|Default|SetbEndSprint true)
          (Ability|RemoveGameplayEffectFromOwnerWithHandle)
          (Ability|EndAbility))))
    (:Is%20Not%20Valid
      (Ability|EndAbility))))

(event Ability|EventOnEndAbility
  (params (bWasCancelled :type Boolean)))

(event EventInputReleased
  (Variables|Default|SetbEndSprint true)
  (Ability|RemoveGameplayEffectFromOwnerWithHandle)
  (Ability|EndAbility))