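; Gameplay ability that makes a spline-based monster dodge left, right or backward, chosen by its CurrentSkillID.
; On activation it turns the skill ID into an actor-relative direction and sets a "Dodge" Motion Warping target a fixed distance from the starting location.
; It then plays a montage and ends the ability when that completes, blends out, is interrupted or is cancelled.
; A leftover DodgeMovement call is never run.
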(event Ability|EventActivateAbility
  (bind _returnvalue (Ability|GetActorInfo))
  (bind _asbpbase_spline_monster (Utilities|Casting|CastToBPBase_SplineMonster (.owneractor _returnvalue)))
  (Variables|Default|SetCurrentSkill_ID (Variables|/Game/Blueprints/10_Monster/BPBase_SplineMonster.BPBase_SplineMonster_C|GetCurrentSkill_ID _asbpbase_spline_monster))
  (Variables|Default|SetFirstLocation (Transformation|GetActorLocation (.owneractor _returnvalue)))
  (switch int (Variables|Default|GetCurrentSkill_ID)
    (:10005
      (Variables|Default|SetDodgeVector (* (Transformation|GetActorRightVector (.owneractor _returnvalue)) -1.0)))
    (:10006
      (bind _output_get (Variables|Default|SetDodgeVector (Transformation|GetActorRightVector (.owneractor _returnvalue)))))
    (:10007
      (Variables|Default|SetDodgeVector (* (Transformation|GetActorForwardVector (.owneractor _returnvalue)) -1.0))))
  (Variables|Default|SetTargetDirection _output_get)
  (Class|MotionWarpingComponent|AddorUpdateWarpTargetfromLocation (Variables|/Game/Blueprints/10_Monster/BPBase_SplineMonster.BPBase_SplineMonster_C|GetMotionWarping _asbpbase_spline_monster) "Dodge" (+ (Variables|Default|GetFirstLocation) (* (Variables|Default|GetTargetDirection) 2e+02)))
  (|PlayMontageandWaitProxy "None" 0 1.0 "None" true 1.0 0.0
    (:OnCompleted
      _)
    (:OnBlendOut
      _)
    (:OnInterrupted
      _)
    (:OnCancelled
      _))
  (Ability|EndAbility))

(event Ability|EventOnEndAbility
  (params (bWasCancelled :type Boolean)))