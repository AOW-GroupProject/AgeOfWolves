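; Gameplay ability for the Wolf monster's dash attack, run on a spline-based monster owner.
; It switches the monster's collision through ChangeCollision while active and restores it when the ability ends.
; A montage drives the attack, and any way it finishes ends the ability.
; A one-shot AttackHit gameplay event reads the Player actor from the AI blackboard, but nothing is done with it yet.
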(event Ability|EventActivateAbility
  (bind _asbpbase_spline_monster (Utilities|Casting|CastToBPBase_SplineMonster (.owneractor (Ability|GetActorInfo))))
  (Default|ChangeCollision _asbpbase_spline_monster false)
  (|PlayMontageandWaitProxy "None" 0 1.0 "None" true 1.0 0.0
    (:then
      (Ability|Tasks|WaitGameplayEvent "(TagName=\"Ability.Monster.AttackHit\")" 0 true
        (:EventReceived
          (Utilities|Casting|CastToActor (AI|Components|Blackboard|GetValueasObject (AI|GetBlackboard (AI|GetAIController _asbpbase_spline_monster)) (Utilities|Name|MakeLiteralName "Player"))))))
    (:OnCompleted
      (Ability|EndAbility :!label _label))
    (:OnBlendOut
      (goto _label))
    (:OnInterrupted
      (goto _label))
    (:OnCancelled
      (goto _label))))

(event Ability|EventOnEndAbility
  (params (bWasCancelled :type Boolean))
  (Default|ChangeCollision (stale Ability|EventActivateAbility _asbpbase_spline_monster) true))