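; BP_LinearTest is a test projectile that delivers Gameplay Ability System effects on hit.
; It takes the player pawn's rotation at BeginPlay.
; A collision hit fires a GameplayCue on the owner and deactivates Niagara; targets with an AbilitySystemComponent receive two GameplayEffects, one via the stored ASC and one self-applied, then the projectile is destroyed.
; Construction-script code for projectile speed and gravity is disconnected and never runs.
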(event OnComponentHit(CollisionComponent)
  (params (HitComponent :type Primitive%20Component%20Object%20Reference) (OtherActor :type Actor%20Object%20Reference) (OtherComp :type Primitive%20Component%20Object%20Reference) (NormalImpulse :type Vector :default "0, 0, 0") (Hit :type Hit%20Result%20Structure%20%28by%20ref%29))
  (bind _returnvalue (Ability|GetAbilitySystemComponent OtherActor))
  (Variables|Default|SetGCNParameter (GameplayCue|MakeGameplayCueParametersfromHitResult (Ability|TargetData|GetHitResultfromTargetData (Ability|TargetData|AbilityTargetDatafromHitResult Hit))))
  (GameplayCue|ExecuteGameplayCueOnActor(Burst) (Components|GetOwner) (Variables|Default|GetGameplayCueTagSpawnProjectile) (Variables|Default|GetGCNParameter))
  (Components|Activation|Deactivate (Variables|Default|GetNiagara))
  (Utilities|IsValid _returnvalue
    (:Is%20Valid
      (GameplayEffects|ApplyGameplayEffectToTarget :self (Variables|Default|GetASC) :GameplayEffectClass (Variables|Default|GetGameplayEffectToApply) :Target _returnvalue)
      (GameplayEffects|ApplyGameplayEffectToSelf :self _returnvalue :GameplayEffectClass (Variables|Default|GetGameplayEfectDamaToHealth))
      (Actor|DestroyActor))))

(event EventBeginPlay
  (Transformation|SetActorRotation (Transformation|GetActorRotation (Game|Player|GetPlayerPawn 0))))

(event Collision|EventActorBeginOverlap
  (params (OtherActor :type Actor%20Object%20Reference)))

(event EventTick
  (params (DeltaSeconds :type Float%20%28single-precision%29)))

(fn ConstructionScript)