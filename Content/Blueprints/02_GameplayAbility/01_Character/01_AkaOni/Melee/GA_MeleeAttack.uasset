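; Gameplay ability for AkaOni's melee katana attack, playing a montage and ending when it completes or is interrupted.
; A looping timer sphere-traces between the blade sockets, passing each hit actor to CauseDamage and adding it to an ignore list.
; A montage gameplay event stops the trace, and ability end clears the list because the ability is instanced per actor.
; Combo-input nodes are present but unconnected.
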(event Custom|Start%20Trace
  ;[1 1 1] 공격 중에 실행되는 Sphere Trace Loop
  (bind _returnvalue (Utilities|Time|SetTimerbyEvent (delegate Custom|Trace%20Loop) 0.05 true))
  (Variables|Default|SetKatanaTraceLoop _returnvalue))

(event Custom|Trace%20Loop
  ;[1 1 1] 공격 중에 실행되는 Sphere Trace Loop
  (bind _outhit (Collision|SphereTraceByChannel (Transformation|GetSocketLocation (Variables|/Script/Engine.Character|GetMesh (Class|AttackGameplayAbility|GetPlayerCharacterfromActorInfo)) "BladeStart") (Transformation|GetSocketLocation (Variables|/Script/Engine.Character|GetMesh (Class|AttackGameplayAbility|GetPlayerCharacterfromActorInfo)) "BladeEnd") (Variables|Default|GetKatanaRadius) "TraceTypeQuery1" false (Variables|Default|GetActorsToIgnore) "ForDuration"))
  (Utilities|Array|AddUnique (Variables|Default|GetActorsToIgnore) (.HitActor (Collision|BreakHitResult _outhit)))
  (Class|AttackGameplayAbility|CauseDamage (.HitActor (Collision|BreakHitResult _outhit))))

(event Custom|Stop%20Trace
  ;[1 1 1] 공격 중에 실행되는 Sphere Trace Loop
  (Utilities|Time|ClearandInvalidateTimerbyHandle (Variables|Default|GetKatanaTraceLoop)))

(event Ability|EventActivateAbility
  (CallFunction|StartTrace)
  (|PlayMontageandWaitProxy "" (Variables|Default|GetMeleeAttackMontage) 1.0 "One" false 1.0 0.0
    (:then
      (Ability|Tasks|WaitGameplayEvent "(TagName=\"Event.Montage.MeleeAttack.End\")" 0
        (:EventReceived
          (CallFunction|StopTrace))))
    (:OnCompleted
      (Ability|EndAbility :!label _label))
    (:OnInterrupted
      (goto _label))
    (:OnCancelled
      (goto _label))))

(event Ability|EventOnEndAbility
  (params (bWasCancelled :type Boolean))
  (bind _actorstoignore (Variables|Default|GetActorsToIgnore))
  ;[1 1 1] Ability의 Instancing Policy가 Instanced Per Actor이기 때문에 이벤트가 종료될 때 초기화 작업을 한다.
  (Development|PrintString "End Ability")
  (Utilities|Array|Clear _actorstoignore)
  (Development|PrintString (Utilities|String|ToString(Integer) (Utilities|Array|Length _actorstoignore))))