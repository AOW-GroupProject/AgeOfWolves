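; AkaOni's normal attack Gameplay Ability: a katana combo played from a single montage, AM_Combo_Full.
; Montage gameplay events start and stop a looping timer that sphere-traces between blade sockets, damaging hit actors and ignoring them until the trace stops.
; A left-click event buffers one follow-up; without it, the ability ends when the current swing's end event arrives.
; As the ability is instanced per actor, OnEndAbility resets input and trace state.
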(event Custom|Attack%20Trace%20Loop
  ;[1 1 1] 공격 중에 실행되는 Sphere Trace Loop
  (bind _outhit (Collision|SphereTraceByChannel (Transformation|GetSocketLocation (Variables|/Script/Engine.Character|GetMesh (Class|AttackGameplayAbility|GetPlayerCharacterfromActorInfo)) "BladeStart") (Transformation|GetSocketLocation (Variables|/Script/Engine.Character|GetMesh (Class|AttackGameplayAbility|GetPlayerCharacterfromActorInfo)) "BladeEnd") (Variables|Default|GetKatanaRadius) "TraceTypeQuery1" false (Variables|Default|GetActorsToIgnore) "ForDuration" true "(R=1.000000,G=0.000000,B=0.000000,A=1.000000)" "(R=0.000000,G=1.000000,B=0.000000,A=1.000000)" 0.5))
  (if (.bBlockingHit (Collision|BreakHitResult _outhit))
    (Utilities|Array|AddUnique (Variables|Default|GetActorsToIgnore) (.HitActor (Collision|BreakHitResult _outhit)))
    (Class|AttackGameplayAbility|CauseDamage (.HitActor (Collision|BreakHitResult _outhit)))))

(event Custom|Stop%20Trace
  ;[1 1 1] 공격 중에 실행되는 Sphere Trace Loop
  (Utilities|Time|ClearandInvalidateTimerbyHandle (Variables|Default|GetKatanaTraceLoop))
  (Utilities|Array|Clear (Variables|Default|GetActorsToIgnore)))

(event Custom|Start%20Attack%20Trace
  ;[1 1 1] 공격 중에 실행되는 Sphere Trace Loop
  (bind _returnvalue (Utilities|Time|SetTimerbyEvent (delegate Custom|Attack%20Trace%20Loop) 0.05 true))
  (Variables|Default|SetKatanaTraceLoop _returnvalue))

(event Ability|EventActivateAbility
  ;[1 1 1] 코멘트
  (Development|PrintString (Utilities|String|ToString(Boolean) (GameplayTags|HasMatchingGameplayTag (Ability|GetAbilitySystemComponentfromActorInfo) "(TagName=\"Ability.Active.Dodge\")")))
  (Utilities|Array|AddUnique (Variables|Default|GetActorsToIgnore) (Class|AttackGameplayAbility|GetPlayerCharacterfromActorInfo))
  (|PlayMontageandWaitProxy "" "/Game/Assets/Aka_Oni/Animation/ComboAttack/AM_Combo_Full.AM_Combo_Full" 1.0 "1" false 1.0 0.0
    (:then
      (Utilities|FlowControl|Sequence
        (:then_0
          (Ability|Tasks|WaitGameplayEvent "(TagName=\"Event.Montage.MeleeAttack.Start\")" 0
            (:EventReceived
              (CallFunction|StartAttackTrace))))
        (:then_1
          (Ability|Tasks|WaitGameplayEvent "(TagName=\"Event.Montage.MeleeAttack.End\")" 0
            (:EventReceived
              (CallFunction|StopTrace)
              (if (== (Variables|Default|GetInputCount) 0)
                (Animation|Montage|MontageStop -1.0)
                (Ability|EndAbility)
                (else
                  (Math|Integer|DecrementInt (Variables|Default|GetInputCount)))))))
        (:then_2
          (Ability|Tasks|WaitGameplayEvent "(TagName=\"Event.MouseLeftInput\")" 0
            (:EventReceived
              (Variables|Default|SetInputCount 1))))))
    (:OnCompleted
      (Ability|EndAbility :!label _label))
    (:OnInterrupted
      (goto _label))
    (:OnCancelled
      (goto _label))))

(event Ability|EventOnEndAbility
  (params (bWasCancelled :type Boolean))
  ;[1 1 1] Ability의 Instancing Policy가 Instanced Per Actor이기 때문에 이벤트가 종료될 때 초기화 작업을 한다.
  (if bWasCancelled
    (Development|PrintString "MeleeAttack Cancel End")
    (else
      (Development|PrintString "MeleeAttack End")))
  (Utilities|Array|Clear (Variables|Default|GetActorsToIgnore))
  (Variables|Default|SetInputCount 0)
  (CallFunction|StopTrace))