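; Melee attack gameplay ability for the AkaOni character that plays a random attack montage and damages what the katana hits.
; A looping timer sphere-traces between blade sockets until a montage-end gameplay event, ignoring the owner and actors already hit.
; Mouse-input events raise a capped combo count, which montage completion decrements to decide whether to end the ability.
; The ignore list is cleared on ability end because the ability is instanced per actor.
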(event Custom|TestLoop
  (Utilities|Time|SetTimerbyEvent (delegate Custom|커스텀이벤트) 0.2 true))

(event Custom|Attack%20Trace%20Loop
  ;[1 1 1] 공격 중에 실행되는 Sphere Trace Loop
  (bind _outhit (Collision|SphereTraceByChannel (Transformation|GetSocketLocation (Variables|/Script/Engine.Character|GetMesh (Class|AttackGameplayAbility|GetPlayerCharacterfromActorInfo)) "BladeStart") (Transformation|GetSocketLocation (Variables|/Script/Engine.Character|GetMesh (Class|AttackGameplayAbility|GetPlayerCharacterfromActorInfo)) "BladeEnd") (Variables|Default|GetKatanaRadius) "TraceTypeQuery1" false (Variables|Default|GetActorsToIgnore) "ForDuration"))
  (if (.bBlockingHit (Collision|BreakHitResult _outhit))
    (Utilities|Array|AddUnique (Variables|Default|GetActorsToIgnore) (.HitActor (Collision|BreakHitResult _outhit)))
    (Class|AttackGameplayAbility|CauseDamage (.HitActor (Collision|BreakHitResult _outhit)))))

(event Custom|Stop%20Trace
  ;[1 1 1] 공격 중에 실행되는 Sphere Trace Loop
  (Utilities|Time|ClearandInvalidateTimerbyHandle (Variables|Default|GetKatanaTraceLoop)))

(event Custom|Start%20Attack%20Trace
  ;[1 1 1] 공격 중에 실행되는 Sphere Trace Loop
  (bind _returnvalue (Utilities|Time|SetTimerbyEvent (delegate Custom|Attack%20Trace%20Loop) 0.05 true))
  (Variables|Default|SetKatanaTraceLoop _returnvalue))

(event Custom|커스텀이벤트
  (Development|PrintString "Loop"))

(event Custom|Increment%20Combo
  (if (< (Variables|Default|GetInputCount) (Variables|Default|GetMaxComboCount))
    (Math|Integer|IncrementInt (Variables|Default|GetInputCount))))

(event Ability|EventActivateAbility
  ;[1 1 1] 코멘트
  (Utilities|Array|AddUnique (Variables|Default|GetActorsToIgnore) (Class|AttackGameplayAbility|GetPlayerCharacterfromActorInfo))
  (CallFunction|StartAttackTrace)
  (|PlayMontageandWaitProxy "" (.OutItem (Utilities|Array|Random (Variables|Default|GetMeleeAttackMontages))) 1.0 "" false 1.0 0.0
    (:then
      (Utilities|FlowControl|Sequence
        (:then_0
          (Ability|Tasks|WaitGameplayEvent "(TagName=\"Event.Montage.MeleeAttack.End\")" 0
            (:EventReceived
              (CallFunction|StopTrace))))
        (:then_1
          (Ability|Tasks|WaitGameplayEvent "(TagName=\"Event.MouseLeftInput\")" 0
            (:EventReceived
              (CallFunction|IncrementCombo))))))
    (:OnCompleted
      (bind _result (Math|Integer|DecrementInt (Variables|Default|GetInputCount))
        (:%20%20
          (if (<= _result 0)
            (Ability|EndAbility)))))
    (:OnInterrupted
      (Ability|EndAbility :!label _label))
    (:OnCancelled
      (goto _label))))

(event Ability|EventOnEndAbility
  (params (bWasCancelled :type Boolean))
  (bind _actorstoignore (Variables|Default|GetActorsToIgnore))
  ;[1 1 1] Ability의 Instancing Policy가 Instanced Per Actor이기 때문에 이벤트가 종료될 때 초기화 작업을 한다.
  (Development|PrintString "End Ability")
  (Utilities|Array|Clear _actorstoignore)
  (Development|PrintString (Utilities|String|ToString(Integer) (Utilities|Array|Length _actorstoignore))))