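; GA_Sprint is a Gameplay Ability that raises its owner's move speed while the sprint input is held, draining stamina.
; Activation requires horizontal movement, then applies GE_Sprint_ChangeMoveSpeed and stores its handle.
; A WaitInputRelease task runs alongside a short WaitDelay loop that commits the ability cost each tick.
; Releasing input, stopping acceleration, falling or failing the cost removes the effect and ends the ability.
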(event Ability|EventActivateAbility
  (bind _returnvalue (Ability|GetActorInfo))
  (bind (_owneractor _avataractor _playercontroller _abilitysystemcomponent _skeletalmeshcomponent _animinstance _movementcomponent) (Utilities|Struct|BreakGameplayAbilityActorInfo _returnvalue))
  ;[1 1 1] #1. Gameplay Ability의 Owner가 현재 어느 방향으로든 이동 중인지 확인합니다.
  (bind _asbase_character_movement_component (Utilities|Casting|CastToBaseCharacterMovementComponent _movementcomponent))
  (Utilities|IsValid _asbase_character_movement_component
    (:Is%20Valid
      ;[1 1 1] #2. GE_Sprint_ChangeMoveSpeed를 Owner에게 적용하고, 그 반환 값을 통해 Active Gameplay Effect Handle을 설정합니다.
      (if (> (Math|Vector|VectorLengthXY (Transformation|GetVelocity _owneractor)) 3.0)
        (bind _returnvalue_2 (Ability|ApplyGameplayEffectToOwner "/Game/Blueprints/02_GameplayAbility/01_Character/01_AkaOni/Sprint/GE_Sprint_ChangeMoveSpeed.GE_Sprint_ChangeMoveSpeed_C" (Ability|GetAbilityLevel)))
        (bind _output_get (Variables|Default|SetGE_Sprint_ChangeMoveSpeed _returnvalue_2))
        ;[1 1 1] #3. Ability Task(Gameplay Ability의 비동기 작업 수행 객체) 중 Wait Input Release를 통해 해당 Gameplay Ability 활성화를 트리거한 Input Key 입력 해제 이벤트를 기다리며, 그 동안에 어떤 작업을 수행할지 정의합니다.
        (Ability|Tasks|WaitInputRelease true
          (:then
            ;[1 1 1] #4. Ability Task(Gameplay Ability의 비동기 작업을 수행하는 객체) 중 Wait Delay(Delay 노드랑 같음) 0.05초 주기로 사용자 Key Input 입력이 해제되지 않았다면,
            ; 해당Gameplay Ability의 Owner의 '이동 중' 여부를 체크하고, 이에 대한 GE_Cost_Sprint_DrainStamina(해당 Gameplay Ability 활성화를 위해 필요한 비용)를 Owner에게 부과해줍니다.
            (Ability|Tasks|WaitDelay 0.05 :!label _label
              (:OnFinish
                (bind _asbase_character_movement_component_2 (Utilities|Casting|CastToBaseCharacterMovementComponent (.movementcomponent (Ability|GetActorInfo))))
                (if (and (> (Math|Vector|VectorLength (Pawn|Components|CharacterMovement|GetCurrentAcceleration _asbase_character_movement_component_2)) 0.0) (not (AI|Components|NavMovement|IsFalling _asbase_character_movement_component_2)))
                  (bind _returnvalue_3 (Ability|CommitAbilityCost false))
                  (if _returnvalue_3
                    (if (Variables|Default|GetbEndSprint)
                      _
                      (else
                        (goto _label)))))
                (Variables|Default|SetbEndSprint true)
                (Ability|RemoveGameplayEffectFromOwnerWithHandle (Variables|Default|GetGE_Sprint_ChangeMoveSpeed))
                (Ability|EndAbility))))
          (:OnRelease
            (Variables|Default|SetbEndSprint true)
            ;;[1 0.04167 0.04167] #5. 종료 조건입니다. Owner의 ASC에 등록되어 있는GE_Sprint_ChangeMoveSpeed 의 ActiveGameplayEffectHandle을 ASC로부터 제거해주어, Owner의 ㅡMoveSpeed 속성의 수치 값을 기존의 값으로 복원해줍니다.
            (Ability|RemoveGameplayEffectFromOwnerWithHandle _output_get)
            (Ability|EndAbility)))
        (else
          (Ability|EndAbility))))))

(event Ability|EventOnEndAbility
  (params (bWasCancelled :type Boolean)))