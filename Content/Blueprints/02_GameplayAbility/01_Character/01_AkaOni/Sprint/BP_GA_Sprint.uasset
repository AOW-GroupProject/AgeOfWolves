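; Sprint gameplay ability for the AkaOni character that raises movement speed while the input is held.
; On activation it casts to BaseCharacterMovementComponent and, only if the owner is moving horizontally, calls ChangeMoveSpeed to the faster sprint speed.
; A WaitInputRelease task then restores the slower speed and ends the ability, while a stationary owner ends it immediately.
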(event Ability|EventActivateAbility
  (bind _returnvalue (Ability|GetActorInfo))
  (bind (_owneractor _avataractor _playercontroller _abilitysystemcomponent _skeletalmeshcomponent _animinstance _movementcomponent) (Utilities|Struct|BreakGameplayAbilityActorInfo _returnvalue))
  (bind _asbase_character_movement_component (Utilities|Casting|CastToBaseCharacterMovementComponent _movementcomponent))
  (Utilities|IsValid _asbase_character_movement_component
    (:Is%20Valid
      (if (> (Math|Vector|VectorLengthXY (Transformation|GetVelocity _owneractor)) 3.0)
        (Class|BaseCharacterMovementComponent|ChangeMoveSpeed _asbase_character_movement_component (Class|MovementComponent|GetMaxSpeed _asbase_character_movement_component) 5e+02)
        (Development|PrintString "Start Sprint")
        (Ability|Tasks|WaitInputRelease true
          (:OnRelease
            (Class|BaseCharacterMovementComponent|ChangeMoveSpeed _asbase_character_movement_component (Class|MovementComponent|GetMaxSpeed _asbase_character_movement_component) 2.3e+02)
            (Development|PrintString "End Srpint")
            (Ability|EndAbility)))
        (else
          (Ability|EndAbility))))))

(event Ability|EventOnEndAbility
  (params (bWasCancelled :type Boolean)))