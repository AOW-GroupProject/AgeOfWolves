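; BP_DefaultPlayerController is a player controller that records movement key input for setting Motion Warping direction.
; Raw W, A, S and D key events add a unit axis offset to InputVector on press and subtract it on release, so held keys combine into a 2D direction.
; The controller only stores the vector; BeginPlay, Tick and the construction script are empty, and a debug print is left disconnected.
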(event EventBeginPlay)

(event EventTick
  (params (DeltaSeconds :type Float%20%28single-precision%29)))

(event Input|KeyboardEvents|W
  (params (Key :type Key%20Structure :default "None"))
  ;[1 1 1] Motion Warping 방향 설정을 위한 입력 저장
  (:Pressed
    (Variables|Default|SetInputVector (+ (Variables|Default|GetInputVector) "(X=0.000000,Y=1.000000)")))
  (:Released
    (Variables|Default|SetInputVector (+ (Variables|Default|GetInputVector) "(X=0.000000,Y=-1.000000)"))))

(event Input|KeyboardEvents|A
  (params (Key :type Key%20Structure :default "None"))
  ;[1 1 1] Motion Warping 방향 설정을 위한 입력 저장
  (:Pressed
    (Variables|Default|SetInputVector (+ (Variables|Default|GetInputVector) "(X=-1.000000,Y=-0.000000)")))
  (:Released
    (Variables|Default|SetInputVector (+ (Variables|Default|GetInputVector) "(X=1.000000,Y=-0.000000)"))))

(event Input|KeyboardEvents|S
  (params (Key :type Key%20Structure :default "None"))
  ;[1 1 1] Motion Warping 방향 설정을 위한 입력 저장
  (:Pressed
    (Variables|Default|SetInputVector (+ (Variables|Default|GetInputVector) "(X=0.000000,Y=-1.000000)")))
  (:Released
    (Variables|Default|SetInputVector (+ (Variables|Default|GetInputVector) "(X=0.000000,Y=1.000000)"))))

(event Input|KeyboardEvents|D
  (params (Key :type Key%20Structure :default "None"))
  ;[1 1 1] Motion Warping 방향 설정을 위한 입력 저장
  (:Pressed
    (Variables|Default|SetInputVector (+ (Variables|Default|GetInputVector) "(X=1.000000,Y=-0.000000)")))
  (:Released
    (Variables|Default|SetInputVector (+ (Variables|Default|GetInputVector) "(X=-1.000000,Y=-0.000000)"))))

(fn ConstructionScript)