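; Base Blueprint for spline monster characters, providing shared turning and movement helpers plus empty combat events for attacks, combos, skills and dodging.
; SetDirToTargetSmoothly uses LookAtTargetLerp, where a timeline scaled to the given duration lerps actor yaw toward the target, only while NextSkillID is within a set limit.
; Helper functions switch the capsule between Pawn and overlap-only collision profiles and set max walk speed.
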(event Custom|SetNextAttackType
  (params (Key :type Name))
  ;[1 1 1] Custom Event - 자식에서 override 해서 사용할 함수
)

(event Custom|BasicAttack
  ;[1 1 1] Custom Event - 자식에서 override 해서 사용할 함수
)

(event Custom|TryActivateSkillAbility
  ;[1 1 1] Custom Event - 자식에서 override 해서 사용할 함수
)

(event Custom|SetDirToTargetSmoothly
  (params (TargetToLookAt :type Actor%20Object%20Reference) (TimelineTime :type Float%20%28double-precision%29))
  ;[1 1 1] SetDirToTarget - 타겟 방향으로 자연스럽게 회전
  (|LookAtTargetLerp TargetToLookAt TimelineTime))

(event Custom|SetNextComboAttack
  ;[1 1 1] Custom Event - 자식에서 override 해서 사용할 함수
)

(event Custom|DodgeMovement
  ;[1 1 1] Custom Event - 자식에서 override 해서 사용할 함수
)

(event EventBeginPlay
  (|CallParentFunction))

(fn ConstructionScript
  (|CallParentFunction))

(fn ChangeCollision
  (params (IsBlock :type Boolean))
  (bind _capsulecomponent (Variables|Default|GetCapsuleComponent))
  (if IsBlock
    (Collision|SetCollisionProfileName _capsulecomponent "Pawn" true :!class /Script/Engine.PrimitiveComponent)
    (else
      (Collision|SetCollisionProfileName _capsulecomponent "OverlapOnlyPawn" true :!class /Script/Engine.PrimitiveComponent))))

(fn ChangeMaxSpeed
  (params (Input :type Float%20%28double-precision%29))
  (Variables|/Script/Engine.CharacterMovementComponent|SetMaxWalkSpeed (Variables|Character|GetCharacterMovement) Input))