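; Base Blueprint for SplineMonster characters, providing skill cooldowns, turning toward a target and empty attack and dodge events for children to override.
; BeginPlay fills a SkillPossibility map from the monster's skill data, which StartSkillCoolDown toggles around a data-driven delay for the availability check to read.
; A timeline-driven macro lerps yaw toward the target, only for NextSkillID up to 10004.
; Helper functions switch capsule collision profiles and set walk speed.
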(event Custom|SetNextAttackType
  (params (Key :type Name))
  ;[1 1 1] Custom Event - 자식에서 override 해서 사용할 함수
)

(event Custom|StartSkillCoolDown
  (params (Skill_ID :type Integer))
  (bind _skillpossibility (Variables|Default|GetSkillPossibility))
  ;[1 1 1] 코멘트
  (Utilities|Map|Add _skillpossibility Skill_ID false)
  (Utilities|FlowControl|Delay (Math|Conversions|ToFloat(Integer) (.skillcooldown (Skill|GetSkillDataThorughID Skill_ID))))
  (Utilities|Map|Add _skillpossibility Skill_ID true))

(event Custom|TryActivateSkillAbility
  ;[1 1 1] Custom Event - 자식에서 override 해서 사용할 함수
)

(event Custom|SetDirToTargetSmoothly
  (params (TargetToLookAt :type Actor%20Object%20Reference) (TimelineTime :type Float%20%28double-precision%29))
  ;[1 1 1] SetDirToTarget - 타겟 방향으로 자연스럽게 회전
  (|LookAtTargetLerp TargetToLookAt TimelineTime))

(event Custom|SetNextComboAttack
  ;[1 1 1] Custom Event - 자식에서 override 해서 사용할 함수
)

(event Custom|BasicAttack
  ;[1 1 1] Custom Event - 자식에서 override 해서 사용할 함수
)

(event Custom|DodgeMovement
  ;[1 1 1] Custom Event - 자식에서 override 해서 사용할 함수
)

(event EventBeginPlay
  (|CallParentFunction)
  ;[1 1 1] 스킬 쿨타임 변수 초기화
  (bind _returnvalue (Class|BaseMonster|GetSingleMonsterData))
  (bind _keys (Utilities|Map|Keys (.monsterskilldata _returnvalue)))
  (for _array_element _keys
    (if (.ReturnValue (Utilities|Map|Find (.monsterskilldata _returnvalue) _array_element))
      (Utilities|Map|Add (Variables|Default|GetSkillPossibility) _array_element true))))

(event EventTick
  (params (DeltaSeconds :type Float%20%28single-precision%29))
  (|CallParentFunction DeltaSeconds))

(fn ConstructionScript
  (|CallParentFunction))

(fn ChangeCollision
  (params (IsBlock :type Boolean))
  (bind _capsulecomponent (Variables|Default|GetCapsuleComponent))
  (if IsBlock
    (Collision|SetCollisionProfileName _capsulecomponent "Pawn" true :!class /Script/Engine.PrimitiveComponent)
    (else
      (Collision|SetCollisionProfileName _capsulecomponent "OverlapOnlyPawn" true :!class /Script/Engine.PrimitiveComponent))))

(fn ChangeMaxSpeed
  (params (Input :type Float%20%28double-precision%29))
  (Variables|/Script/Engine.CharacterMovementComponent|SetMaxWalkSpeed (Variables|Character|GetCharacterMovement) Input))

(fn GetSkillDataThorughID
  (params (InputID :type Integer))
  (bind _returnvalue (Class|BaseMonster|GetSingleMonsterData))
  (if (.ReturnValue (Utilities|Map|Find (.monsterskilldata _returnvalue) InputID))
    (return (.Value (Utilities|Map|Find (.monsterskilldata _returnvalue) InputID)))
    (else
      (return ""))))

(fn IsPossibleSkillCoolDown
  (params (Skill_ID :type Integer))
  (bind _skillpossibility (Variables|Default|GetSkillPossibility))
  (bind (_value _returnvalue) (Utilities|Map|Find _skillpossibility Skill_ID))
  (if _returnvalue
    (if _value
      (return true)
      (else
        _)))
  (return false))