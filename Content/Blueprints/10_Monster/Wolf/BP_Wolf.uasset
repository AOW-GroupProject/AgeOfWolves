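; Wolf monster that fights through Gameplay Ability System skills: basic attacks, a dash and directional dodges.
; Skill selection uses cooldowns and random rolls, writing the chosen skill's max range to the blackboard.
; Skills activate by data-driven tags, start cooldowns and can chain into linked combo skills by probability.
; Dash lerps toward the target unless blocked, dodges set motion-warp targets, and capsule traces send hit events.
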(event Custom|StartSkillCoolDown
  (params (Skill_ID :type Integer))
  ;[1 1 1] 스킬 쿨타임
  (Utilities|Map|Add (Variables|SkillData|GetSkillPossibility) Skill_ID false)
  (Utilities|FlowControl|Delay (Math|Conversions|ToFloat(Integer) (.skillcooldown (SkillData|GetSkillDataThroughID Skill_ID))))
  (Utilities|Map|Add (Variables|SkillData|GetSkillPossibility) Skill_ID true))

(event Custom|DashMovement
  (bind __target (Target|GetTarget))
  ;[1 1 1] DashAttackMovement  - 돌진공격 움직임
  (Utilities|IsValid __target
    (:Is%20Valid
      (Variables|DashAttack|SetFirstLocation (Transformation|GetActorLocation))
      (Variables|DashAttack|SetTargetDirection (Class|KismetMathLibrary|VectorNormal2D (- (Transformation|GetActorLocation __target) (Transformation|GetActorLocation)) 0.0001))
      (bind _newtrack_0 (Timeline|DashTimeline PlayFromStart)
        (:Update
          (if (not (DashAttack|IsCollisionFront))
            (Transformation|SetActorLocation (Math|Vector|Lerp(Vector) (Variables|DashAttack|GetFirstLocation) (+ (Variables|DashAttack|GetFirstLocation) (* (Variables|DashAttack|GetTargetDirection) 6e+02)) _newtrack_0) false false)))))))

(event EventBeginPlay
  (|CallParentFunction)
  (CallFunction|GiveAbility)
  (bind _returnvalue (Class|BaseMonster|GetSingleMonsterData))
  (bind _keys (Utilities|Map|Keys (.monsterskilldata _returnvalue)))
  (for _array_element _keys
    (if (.ReturnValue (Utilities|Map|Find (.monsterskilldata _returnvalue) _array_element))
      (Utilities|Map|Add (Variables|SkillData|GetSkillPossibility) _array_element true))))

(event Collision|EventActorBeginOverlap
  (params (OtherActor :type Actor%20Object%20Reference))
  (|CallParentFunction OtherActor))

(event EventTick
  (params (DeltaSeconds :type Float%20%28single-precision%29))
  (|CallParentFunction DeltaSeconds))

(event EventBasicAttack
  ;[1 1 1] BasicAttack_Apply Damage - Trace로 BasicAttack 대상 탐색
  (|BasicAttack_ApplyDamage))

(event EventSetNextAttackType
  (params (Key :type Name :default "None"))
  ;[1 1 1] SetNextAttack - 다음 공격 정하기
  (bind _maxdistance (|SetNextAttackFlow)
    (:WhenReturnValue
      (AI|Components|Blackboard|SetValueasFloat (AI|GetBlackboard (Pawn|GetController)) Key _maxdistance))))

(event EventTryActivateSkillAbility
  ;[1 1 1] TryActivateSkillAbility - 실행할 스킬어빌리티를 Tag로 활성화 시도
  (|TrySkillAbilityByTag))

(event EventSetNextComboAttack
  ;[1 1 1] SetNextComboAttack - 다음 연계 스킬을 정해줌. Notify에서 실행
  (|SetNextComboAttackTypeByCurrentSkill))

(event EventDodgeMovement
  ;[1 1 1] Dodge - 회피
  (Variables|DashAttack|SetFirstLocation (Transformation|GetActorLocation))
  (switch int (Variables|Default|GetCurrentSkill_ID)
    (:10005
      (Variables|Default|SetDodgeVector (* (Transformation|GetActorRightVector) -1.0)))
    (:10006
      (bind _output_get (Variables|Default|SetDodgeVector (Transformation|GetActorRightVector))))
    (:10007
      (Variables|Default|SetDodgeVector (* (Transformation|GetActorForwardVector) -1.0))))
  (Variables|DashAttack|SetTargetDirection _output_get)
  (Class|MotionWarpingComponent|AddorUpdateWarpTargetfromLocation (Variables|Default|GetMotionWarping) "Dodge" (+ (Variables|DashAttack|GetFirstLocation) (* (Variables|DashAttack|GetTargetDirection) 2e+02))))

(fn ConstructionScript
  (|CallParentFunction))

(fn ANFuncDashAttack
  (CallFunction|DashMovement))

(fn GetTarget
  (bind _asactor (Utilities|Casting|CastToActor (AI|Components|Blackboard|GetValueasObject (AI|GetBlackboard (AI|GetAIController self)) (Utilities|Name|MakeLiteralName "Player"))))
  (return _asactor))

(fn IsCollisionFront
  (bind _returnvalue (Transformation|GetActorLocation))
  (bind _returnvalue_2 (Collision|MultiLineTraceByChannel _returnvalue (+ _returnvalue (* (Variables|DashAttack|GetTargetDirection) 1.5e+02)) "TraceTypeQuery3" false 0 "None"))
  (return _returnvalue_2))

(fn GiveAbility
  (bind _abilitysystemcomponent (Variables|Default|GetAbilitySystemComponent))
  (GameplayAbilities|GiveAbility _abilitysystemcomponent "/Game/Blueprints/02_AbilitySystem/02_Monster/GA_MonsterBasicAttack_2.GA_MonsterBasicAttack_2_C" 0 -1)
  (GameplayAbilities|GiveAbility _abilitysystemcomponent "/Game/Blueprints/02_AbilitySystem/02_Monster/GA_MonsterBasicAttack_3.GA_MonsterBasicAttack_3_C" 0 -1)
  (GameplayAbilities|GiveAbility _abilitysystemcomponent "/Game/Blueprints/02_AbilitySystem/02_Monster/GA_MonsterDashAttack.GA_MonsterDashAttack_C" 0 -1)
  (GameplayAbilities|GiveAbility _abilitysystemcomponent "/Game/Blueprints/02_AbilitySystem/02_Monster/GA_MonsterDodge_Back.GA_MonsterDodge_Back_C" 0 -1)
  (GameplayAbilities|GiveAbility _abilitysystemcomponent "/Game/Blueprints/02_AbilitySystem/02_Monster/GA_MonsterDodge_Left.GA_MonsterDodge_Left_C" 0 -1)
  (GameplayAbilities|GiveAbility _abilitysystemcomponent "/Game/Blueprints/02_AbilitySystem/02_Monster/GA_MonsterDodge_Right.GA_MonsterDodge_Right_C" 0 -1)
  (GameplayAbilities|GiveAbility (Variables|Default|GetAbilitySystemComponent) "/Game/Blueprints/02_AbilitySystem/02_Monster/GA_MonsterBasicAttack_1.GA_MonsterBasicAttack_1_C" 0 -1))

(fn GetSkillDataThroughID
  (params (ID :type Integer))
  (bind _returnvalue (Class|BaseMonster|GetSingleMonsterData))
  (if (.ReturnValue (Utilities|Map|Find (.monsterskilldata _returnvalue) ID))
    (return (.Value (Utilities|Map|Find (.monsterskilldata _returnvalue) ID)))
    (else
      (return ""))))

(fn IsPossibleSkillCoolDown
  (params (Skill_ID :type Integer))
  (bind _skillpossibility (Variables|SkillData|GetSkillPossibility))
  (bind (_value _returnvalue) (Utilities|Map|Find _skillpossibility Skill_ID))
  (if _returnvalue
    (if _value
      (return true)
      (else
        _)))
  (return false))

(fn IsCollisionAnywhere
  (bind _returnvalue (Transformation|GetActorLocation))
  (bind _returnvalue_2 (Collision|MultiLineTraceByChannel _returnvalue (+ _returnvalue (* (Variables|DashAttack|GetTargetDirection) 9e+01)) "TraceTypeQuery3" false 0 "ForDuration"))
  (if _returnvalue_2
    (return true)
    (else
      (return false))))

(fn IsWallwhenDodge
  (params (ID :type Integer))
  (switch int ID))